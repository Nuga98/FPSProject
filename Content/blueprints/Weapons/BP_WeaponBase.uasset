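; BP_WeaponBase is a weapon base Blueprint that handles magazine and reserve ammo bookkeeping.
; WeaponFire removes one round from the magazine without checking bounds, and two query functions report magazine and reserve status.
; WeaponReload sets the magazine to the lesser of capacity and reserve and deducts that amount, discarding any rounds still loaded.
; The event graph and construction script hold no logic.
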(event EventBeginPlay)

(event Collision|EventActorBeginOverlap
  (params (OtherActor :type Actor%20Object%20Reference)))

(event EventTick
  (params (DeltaSeconds :type Float%20%28single-precision%29)))

(fn ConstructionScript)

(fn WeaponFire
  (Variables|Default|SetCurrentAmmo (- (Variables|Default|GetCurrentAmmo) 1)))

(fn WeaponReload
  (Variables|Default|SetCurrentAmmo (Math|Integer|Min(Integer) (Variables|Default|GetMaxMagAmmo) (Variables|Default|GetCurrentTotalAmmo)))
  (Variables|Default|SetCurrentTotalAmmo (- (Variables|Default|GetCurrentTotalAmmo) (Math|Integer|Min(Integer) (Variables|Default|GetMaxMagAmmo) (Variables|Default|GetCurrentTotalAmmo)))))

(fn HasAmmoinMag
  (return (> (Variables|Default|GetCurrentAmmo) 0) (== (Variables|Default|GetCurrentAmmo) (Variables|Default|GetMaxMagAmmo))))

(fn HasExtraAmmo
  (return (> (Variables|Default|GetCurrentTotalAmmo) 0)))